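; Behavior tree condition that passes when the AI pawn has line of sight to the blackboard Target actor within a view angle.
; It line traces from a forward offset of the pawn to the Target, ignoring all PickableItemBase actors and drawing debug lines.
; If the trace hits the Target, it compares the arccosine of forward dot direction against AngleVision.
; The direction vector is not normalized before the dot product.
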(fn `PerformConditionCheckAI`
  (params (OwnerController :type "AIController Object Reference") (ControlledPawn :type "Pawn Object Reference"))
  (returns (ReturnValue :type Boolean))
  (bind _outactors (`GameplayStatics.GetAllActorsOfClass` "/Script/Project.PickableItemBase"))
  (bind _asactor (cast `Actor` (`BTFunctionLibrary.GetBlackboardValueAsObject` (`self.Target`)))
    (:`then`
      (bind _outhit (`KismetSystemLibrary.LineTraceSingle` (+ (`Actor.K2_GetActorLocation` ControlledPawn) (* (`Actor.GetActorForwardVector` ControlledPawn) (`self.Offset`))) (`Actor.K2_GetActorLocation` _asactor) "TraceTypeQuery3" false _outactors "ForDuration"))
      (if (== (`.HitActor` (`GameplayStatics.BreakHitResult` _outhit)) _asactor)
        (return (< (`KismetMathLibrary.DegAcos` (`KismetMathLibrary.Dot_VectorVector` (`Actor.GetActorForwardVector` ControlledPawn) (- (`Actor.K2_GetActorLocation` _asactor) (`Actor.K2_GetActorLocation` ControlledPawn)))) (`self.AngleVision`)))
        (else
          (return false))))
    (:`CastFailed`
      (return false))))