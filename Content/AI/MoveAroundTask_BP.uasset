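; Behavior tree task that moves the controlled pawn around the actor stored in a blackboard key, in one angular step.
; It rotates the pawn's offset from that actor by a yaw step angle, randomly adjusted, and sends the pawn there with AI MoveTo.
; Tick finishes with success within an acceptable distance of the destination, or failure when the pawn nearly stops.
; A missing target or failed move also fails the task.
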(event `self.ReceiveExecuteAI`
  (params (OwnerController :type "AIController Object Reference") (ControlledPawn :type "Pawn Object Reference"))
  (bind _asactor (cast `Actor` (`BTFunctionLibrary.GetBlackboardValueAsObject` (`self.TargetKey`)))
    (:`then`
      (if (`KismetMathLibrary.RandomBool`)
        (`/Engine/EditorBlueprintResources/StandardMacros.NegateFloat` (`self.StepAngle`)
          (:`  `
            _)))
      (bind _returnvalue (`Actor.K2_GetActorLocation` _asactor))
      (bind _output_get (set `self.ResultVec` (+ (`KismetMathLibrary.GreaterGreater_VectorRotator` (- (`Actor.K2_GetActorLocation` ControlledPawn) _returnvalue) (`KismetMathLibrary.MakeRotator` 0.0 0.0 (`self.StepAngle`))) _returnvalue)))
      (`|AIMoveTo` ControlledPawn _output_get null 20.0
        (:`OnFail`
          (`self.FinishExecute` false))))
    (:`CastFailed`
      (`self.FinishExecute` false))))

(event `self.ReceiveTickAI`
  (params (OwnerController :type "AIController Object Reference") (ControlledPawn :type "Pawn Object Reference") (DeltaSeconds :type "Float (single-precision)"))
  (`|ExecutionSequence`
    (:`then_0`
      (if (< (`KismetMathLibrary.VSize` (`Actor.GetVelocity` ControlledPawn)) 10.0)
        (`self.FinishExecute` false)))
    (:`then_1`
      (if (< (`KismetMathLibrary.VSize` (- (`self.ResultVec`) (`Actor.K2_GetActorLocation` ControlledPawn))) (`self.AcceptableDistance`))
        (`self.FinishExecute` true)))))