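; Behavior Tree task that keeps the controlled pawn at a Blackboard-defined distance from a target actor.
; On execute it moves along the line to the target by the distance error, clamped to one step, succeeding immediately if that step is within tolerance.
; Tick ends the task, failing when the pawn is nearly stationary and succeeding near the computed location.
; It also fails when the target key holds no actor.
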(event `self.ReceiveExecuteAI`
  (params (OwnerController :type "AIController Object Reference") (ControlledPawn :type "Pawn Object Reference"))
  (bind _stepdistance (`self.StepDistance`))
  (set `self.CurrentLocation` (`Actor.K2_GetActorLocation` ControlledPawn))
  (bind _asactor (cast `Actor` (`BTFunctionLibrary.GetBlackboardValueAsObject` (`self.TargetKey`)))
    (:`then`
      (set `self.TargetLocation` (`Actor.K2_GetActorLocation` _asactor))
      (bind _output_get (set `self.CurrentDistance` (`Actor.GetDistanceTo` ControlledPawn _asactor)))
      (bind _returnvalue (`KismetMathLibrary.FClamp` (- _output_get (`BTFunctionLibrary.GetBlackboardValueAsFloat` (`self.DistanceKey`))) (* _stepdistance -1.0) _stepdistance))
      (bind _returnvalue_2 (+ (* (`KismetMathLibrary.GetDirectionVector` (`self.CurrentLocation`) (`self.TargetLocation`)) _returnvalue) (`self.CurrentLocation`)))
      (set `self.ResultLocation` _returnvalue_2)
      (if (> (`KismetMathLibrary.Abs` _returnvalue) (`self.AcceptanceDistance`))
        (`|AIMoveTo` ControlledPawn _returnvalue_2 null 20.0)
        (else
          (`self.FinishExecute` true))))
    (:`CastFailed`
      (`self.FinishExecute` false))))

(event `self.ReceiveTickAI`
  (params (OwnerController :type "AIController Object Reference") (ControlledPawn :type "Pawn Object Reference") (DeltaSeconds :type "Float (single-precision)"))
  (`|ExecutionSequence`
    (:`then_0`
      (if (< (`KismetMathLibrary.VSize` (`Actor.GetVelocity` ControlledPawn)) 10.0)
        (`self.FinishExecute` false)))
    (:`then_1`
      (if (< (`KismetMathLibrary.VSize` (- (`self.ResultLocation`) (`Actor.K2_GetActorLocation` ControlledPawn))) (`self.AcceptanceDistance`))
        (`self.FinishExecute` true)))))