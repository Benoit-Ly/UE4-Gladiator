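; Behavior tree task that moves the controlled pawn to a blackboard target actor and can be interrupted by a blackboard condition.
; On execute it runs AI MoveTo toward the TargetKey actor, finishing with the move's result, or failing if the value is not an actor.
; Each tick it fails the task when the ConditionKey bool is false, without explicitly stopping the move.
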(event `self.ReceiveExecuteAI`
  (params (OwnerController :type "AIController Object Reference") (ControlledPawn :type "Pawn Object Reference"))
  (bind _asactor (cast `Actor` (`BTFunctionLibrary.GetBlackboardValueAsObject` (`self.TargetKey`)))
    (:`then`
      (`|AIMoveTo` ControlledPawn (0.0 0.0 0.0) _asactor (`self.AcceptanceRadius`)
        (:`OnSuccess`
          (`self.FinishExecute` true))
        (:`OnFail`
          (`self.FinishExecute` false))))
    (:`CastFailed`
      (`self.FinishExecute` false))))

(event `self.ReceiveTickAI`
  (params (OwnerController :type "AIController Object Reference") (ControlledPawn :type "Pawn Object Reference") (DeltaSeconds :type "Float (single-precision)"))
  (if (not (`BTFunctionLibrary.GetBlackboardValueAsBool` (`self.ConditionKey`)))
    (`self.FinishExecute` false)))