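; Pickable war hammer weapon actor that plays a collision sound when it strikes something.
; The construction script assigns its components to mesh, proximity sphere and damage box variables, likely inherited from a shared pickable weapon parent.
; A hit on the Cube component plays the weapon collision cue at the impact point.
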(event `self.Cube.OnComponentHit`
  (params (HitComponent :type "PrimitiveComponent Object Reference") (OtherActor :type "Actor Object Reference") (OtherComp :type "PrimitiveComponent Object Reference") (NormalImpulse :type "Vector Structure") (Hit :type "HitResult Structure (by ref)"))
  (`GameplayStatics.PlaySoundAtLocation` "/Game/Sounds/Weapons/WeaponColisionCue.WeaponColisionCue" (`.Location` (`GameplayStatics.BreakHitResult` Hit))))

(fn `UserConstructionScript`
  (`|ExecutionSequence`
    (:`then_0`
      (set `self.StaticMesh` (`self.Cube`)))
    (:`then_1`
      (set `self.Mesh` (`self.WarHammer`)))
    (:`then_2`
      (set `self.ProxSphere` (`self.Sphere`)))
    (:`then_3`
      (set `self.DamageBox` (`self.CubeCollider`)))))