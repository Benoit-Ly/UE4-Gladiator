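; Game state Blueprint for the ArenaFight mode that relays level win, lose and restart events between the game mode and listeners.
; On BeginPlay the authority caches the ArenaFight game mode, with debug prints for server and client.
; Authority-only events forward no-player-left, no-opponent-left and restart requests to the game mode.
; Losing also sets GameOver, and loss and restart fire validate events that call matching dispatchers.
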(event `self.ReceiveBeginPlay`
  (`/Engine/EditorBlueprintResources/ActorMacros.Switch Has Authority`
    (:`Authority`
      (bind _asarena_fight_game_mode_bp (cast `/Game/Blueprints/ArenaFight_GameModeBP` (`self.AuthorityGameMode`))
        (:`then`
          (set `self.ArenaFightGameMode` _asarena_fight_game_mode_bp)
          (`KismetSystemLibrary.PrintString` "YOU HAVE AUTHORITY" false true (struct :`R` 1.0 :`G` 0.023671 :`A` 1.0) 60.0))
        (:`CastFailed`
          (`KismetSystemLibrary.PrintString` "Couldn't cast from GameMode to ArenaFight_GameModeBP" false))))
    (:`Remote`
      (`KismetSystemLibrary.PrintString` "YOU ARE CLIENT" false true (struct :`R` 0.028321 :`B` 1.0 :`A` 1.0) 60.0))))

(event `self.OnNoPlayerLeft`
  ;[1 1 1] Events for triggering Level Ending
  (`/Engine/EditorBlueprintResources/ActorMacros.Switch Has Authority`
    (:`Authority`
      (`/Game/Blueprints/ArenaFight_GameModeBP.OnLoseLevel_Event` (`self.ArenaFightGameMode`))
      (set `self.bGameOver` true)
      (`self.OnLoseValidate_Event`))))

(event `self.OnNoOpponentLeft`
  ;[1 1 1] Events for triggering Level Ending
  (`/Engine/EditorBlueprintResources/ActorMacros.Switch Has Authority`
    (:`Authority`
      (`/Game/Blueprints/ArenaFight_GameModeBP.OnWinLevel_Event` (`self.ArenaFightGameMode`)))))

(event `self.OnRestartRequest`
  ;[1 1 1] Events for triggering Level Ending
  (`/Engine/EditorBlueprintResources/ActorMacros.Switch Has Authority`
    (:`Authority`
      (`/Game/Blueprints/ArenaFight_GameModeBP.RequestRestart` (`self.ArenaFightGameMode`))
      (`self.OnRestartValidate_Event`))))

(event `OnLoseValidate_Event`
  ;[1 1 1] Events for triggering Level Ending
  (`self.OnLoseValidate`))

(event `OnRestartValidate_Event`
  ;[1 1 1] Events for triggering Level Ending
  (`self.OnRestartValidate`))

(fn `UserConstructionScript`)