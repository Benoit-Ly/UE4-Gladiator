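; Game mode for an arena fight that handles level win and loss and multiplayer restarts.
; Winning starts the next wave, while losing fires the lose-level dispatcher, each with a debug print.
; RequestRestart runs only with authority, passing the current level name to GetServerTravelCommand, executing the result as a console command and firing the restart dispatcher.
; GetServerTravelCommand contains only an unconnected string append for a listen-server travel command.
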(event `OnWinLevel_Event`
  ;[1 1 1] Events when Game needs to end
  (`KismetSystemLibrary.PrintString` "Player has won!" true true (struct :`R` 1.0 :`G` 0.018245 :`A` 1.0) 50.0)
  (`self.StartNextWave`))

(event `OnLoseLevel_Event`
  ;[1 1 1] Events when Game needs to end
  (`KismetSystemLibrary.PrintString` "Player has lost!" true true (struct :`R` 1.0 :`B` 0.015782 :`A` 1.0) 50.0)
  (`self.OnLoseLevel`))

(fn `RequestRestart`
  (`/Engine/EditorBlueprintResources/ActorMacros.Switch Has Authority`
    (:`Authority`
      (bind _returnvalue (`GameplayStatics.GetCurrentLevelName` true))
      (bind _fullcommand (`self.GetServerTravelCommand` _returnvalue))
      (`KismetSystemLibrary.PrintString` _fullcommand)
      (`KismetSystemLibrary.ExecuteConsoleCommand` _fullcommand)
      (`self.OnRestart`))
    (:`Remote`
      (`KismetSystemLibrary.PrintString` "No authority"))))

(fn `UserConstructionScript`)